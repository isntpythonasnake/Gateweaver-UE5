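; BP_CubeSpawner is an actor that spawns and destroys a single tracked BP_CubePawn.
; SpawnCube destroys any existing pawn, spawns a replacement at the SpawnPoint transform regardless of collision, and sets its Cube component's world scale from CubeScale.
; DestroyCube removes the tracked pawn if valid.
; SendCubeSpawnedEvent calls the CubeIsCreated dispatcher, but SpawnCube does not invoke it.
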(event Custom|SpawnCube
  (Utilities|IsValid (Variables|Default|GetBP_CubePawn)
    (:Is%20Valid
      (Actor|DestroyActor (Variables|Default|GetBP_CubePawn)))
    (:Is%20Not%20Valid
      _))
  (bind _returnvalue (Game|SpawnActorfromClass "/Gateweaver-PMS_v2/Actors/BP_CubePawn.BP_CubePawn_C" (Transformation|GetWorldTransform (Variables|Default|GetSpawnPoint)) "AlwaysSpawn" "MultiplyWithRoot" 0 0))
  (bind _output_get (Variables|Default|SetBP_CubePawn _returnvalue))
  (Transformation|SetWorldScale3D (Variables|/Gateweaver-PMS_v2/Actors/BP_CubePawn.BP_CubePawn_C|GetCube _output_get) (Math|Conversions|ToVector(Float) (Variables|Default|GetCube%20Scale))))

(event Custom|DestroyCube
  (Utilities|IsValid (Variables|Default|GetBP_CubePawn)
    (:Is%20Valid
      (Actor|DestroyActor (Variables|Default|GetBP_CubePawn)))))

(fn ConstructionScript)

(fn SendCubeSpawnedEvent
  (params (Cube%20Spawned :type BP%20Cube%20Pawn%20Object%20Reference))
  (Default|CallCubeIsCreated Cube%20Spawned))
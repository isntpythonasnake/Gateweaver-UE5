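; Box trigger volume that switches linked portals on or off when the player character overlaps it.
; Exit triggers disable the linked portals, while Enter triggers enable them and restore each to its original transform.
; Triggers not flagged single-use also disable a separate list of portals to remove first.
; Every overlap also forces the player capsule to block a custom trace channel, as a workaround for walls not blocking collisions.
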(event OnComponentBeginOverlap(Box)
  (params (OverlappedComponent :type Primitive%20Component%20Object%20Reference) (OtherActor :type Actor%20Object%20Reference) (OtherComp :type Primitive%20Component%20Object%20Reference) (OtherBodyIndex :type Integer) (bFromSweep :type Boolean) (SweepResult :type Hit%20Result%20Structure%20%28by%20ref%29))
  (bind _returnvalue (Game|GetPlayerCharacter 0))
  ;[0.1406 0 0 0.5] Had an issue with walls not blocking collisions. This seems to fix it I've no idea why it wasn't blocked by default.
  (Collision|SetCollisionResponsetoChannel (Variables|/Script/Engine.Character|GetCapsuleComponent _returnvalue) "ECC_GameTraceChannel2" "ECR_Block")
  (if (== OtherActor _returnvalue)
    (if (Variables|Setup|GetbIsSingleUse?)
      _
      (else
        (for _array_element (Variables|NotSingle|GetPortalsToRemove)
          (Default|DisablePortals _array_element))))
    (for _array_element_2 (Variables|YesSingle|GetPortals%20Linked)
      (switch Utilities|FlowControl|Switch|SwitchonEnum_ExitOrEnter (Variables|Setup|GetType%20of%20Trigger)
        (:NewEnumerator0
          (Default|DisablePortals _array_element_2))
        (:NewEnumerator1
          (Default|EnablePortals _array_element_2)
          (Transformation|SetActorTransform _array_element_2 (Variables|/Game/Base/Plugin/PortalSource/Plugin/BP_Portal.BP_Portal_C|GetOriginalTransform _array_element_2)))))))

(fn ConstructionScript)
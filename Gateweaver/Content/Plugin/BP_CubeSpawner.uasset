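; Spawner Blueprint that keeps track of a single BP_CubePawn and creates or removes it on demand.
; SpawnCube destroys any valid existing pawn, then always spawns a replacement at the SpawnPoint transform and stores the reference.
; DestroyCube removes the stored pawn if it is valid.
; SendCubeSpawnedEvent forwards a cube to CubeIsCreated, but neither event in the graph calls it.
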(event Custom|SpawnCube
  ;[0 0 0 0.5] Literally just spawns a cube and destroys the existing cube if it exists.
  (Utilities|IsValid (Variables|Default|GetBP_CubePawn)
    (:Is%20Valid
      (Actor|DestroyActor (Variables|Default|GetBP_CubePawn)))
    (:Is%20Not%20Valid
      _))
  (bind _returnvalue (Game|SpawnActorfromClass "/Gateweaver-PMS_v2/Plugin/BP_CubePawn.BP_CubePawn_C" (Transformation|GetWorldTransform (Variables|Default|GetSpawnPoint)) "AlwaysSpawn" "MultiplyWithRoot" 0 0))
  (Variables|Default|SetBP_CubePawn _returnvalue))

(event Custom|DestroyCube
  ;[0 0 0 0.5] Literally just spawns a cube and destroys the existing cube if it exists.
  (Utilities|IsValid (Variables|Default|GetBP_CubePawn)
    (:Is%20Valid
      (Actor|DestroyActor (Variables|Default|GetBP_CubePawn)))))

(fn ConstructionScript)

(fn SendCubeSpawnedEvent
  (params (Cube%20Spawned :type BP%20Cube%20Pawn%20Object%20Reference))
  (Default|CallCubeIsCreated Cube%20Spawned))
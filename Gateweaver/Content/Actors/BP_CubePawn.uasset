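; BP_CubePawn is a cube the player picks up with a long interaction, also used in a boss fight.
; On start it moves to a computed location, attaches to the player character and ignores Pawn collision; cancelling detaches it and restores physics, gravity and blocking.
; The author notes that the snap location is sometimes wrong.
; It announces its spawn on BeginPlay, and its overlap area sends destroy messages to BPI_Destructible actors.
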(event OnLongInteraction(InteractionComponent)
  (params (Instigator :type Actor%20Object%20Reference) (Phase :type InteractionPhase%20Enum :default "NewEnumerator0") (Delta :type Float%20%28double-precision%29))
  (bind _cube (Variables|Default|GetCube))
  ;[0 0 0 0.5] Allows pickup of cube. unfrotunately the location the cube snaps to on the player isn't always the right one. i'm still not sure how to fix this sorry
  (switch Utilities|FlowControl|Switch|SwitchonInteractionPhase Phase
    (:NewEnumerator0
      (Transformation|SetActorLocation (|CollapseGraph) false false)
      (Transformation|AttachActorToActor (Game|GetPlayerCharacter 0) "None" "KeepWorld" "KeepWorld" "KeepRelative" true)
      (Collision|SetCollisionResponsetoChannel (Variables|Default|GetCube) "ECC_Pawn" "ECR_Ignore"))
    (:NewEnumerator3
      (Physics|SetSimulatePhysics _cube true)
      (Physics|SetEnableGravity _cube true)
      (Transformation|DetachFromActor "KeepRelative" "KeepRelative" "KeepRelative")
      (Collision|SetCollisionResponsetoAllChannels _cube "ECR_Block"))))

(event OnComponentBeginOverlap(OverlapArea)
  (params (OverlappedComponent :type Primitive%20Component%20Object%20Reference) (OtherActor :type Actor%20Object%20Reference) (OtherComp :type Primitive%20Component%20Object%20Reference) (OtherBodyIndex :type Integer) (bFromSweep :type Boolean) (SweepResult :type Hit%20Result%20Structure%20%28by%20ref%29))
  ;[0.15 0 0 0.5] This is for my boss fight so ignore this
  (if (Utilities|DoesObjectImplementInterface OtherActor "/Gateweaver-PMS_v2/Interfaces/BPI_Destructible.BPI_Destructible_C")
    (Class|BPIDestructible|Destroy(Message) OtherActor (.ImpactPoint (Collision|BreakHitResult SweepResult)))))

(event EventBeginPlay
  (Collision|SetCollisionResponsetoChannel (Variables|Default|GetCube) "ECC_GameTraceChannel2" "ECR_Block")
  (Default|CallCubeIsSpawned))

(fn ConstructionScript
  (Collision|SetCollisionResponsetoChannel (Variables|Default|GetCube) "ECC_GameTraceChannel2" "ECR_Block"))
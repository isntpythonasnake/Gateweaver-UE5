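; BP_LevelTrigger is a box trigger that sets up or shuts down a level's portals when the player overlaps it.
; It rescans all portals on each overlap and, unless JustSpawnPortals is set, disables those outside PortalsToActivate.
; Listed portals are disabled on Exit, or enabled with their original transforms restored on Enter.
; Optional flags destroy the spawner's cube and drop the portal gun, returning it to its original transform.
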(event OnComponentBeginOverlap(Box)
  (params (OverlappedComponent :type Primitive%20Component%20Object%20Reference) (OtherActor :type Actor%20Object%20Reference) (OtherComp :type Primitive%20Component%20Object%20Reference) (OtherBodyIndex :type Integer) (bFromSweep :type Boolean) (SweepResult :type Hit%20Result%20Structure%20%28by%20ref%29))
  (bind _returnvalue (Game|GetPlayerCharacter 0))
  ;[0.1406 0 0 0.5] Had an issue with walls not blocking collisions. This seems to fix it I've no idea why it wasn't blocked by default.
  (Collision|SetCollisionResponsetoChannel (Variables|/Script/Engine.Character|GetCapsuleComponent _returnvalue) "ECC_GameTraceChannel2" "ECR_Block")
  (if (== OtherActor _returnvalue)
    ;[0 0 0 0.5] Re-run the function to account for newly spawned portals from gun
    (CallFunction|GetAllPortalsinScene)
    (Utilities|FlowControl|Sequence
      (:then_0
        ;[0 0 0 0.5] Is the trigger to destroy any spawned cubes in the level?
        (if (Variables|HasCubeSpawner?|GetbHasCubeSpawner?)
          (bind _bp_cubespawner (Variables|HasCubeSpawner?|GetBP_CubeSpawner)
            (:then
              (Default|DestroyCube _bp_cubespawner))
            (:else
              _)))
        ;[0 0 0 0.5] I'm not quite sure what to name this boolean. My english isn't working today.
        (if (Variables|Setup|GetbJustSpawnPortals?)
          _
          (else
            ;[0 0 0 0.5] If trigger is to remove other portals, ie portals that teleport player into the level
            (for _array_element (Variables|Internal|GetFilteredPortals)
              (Default|DisablePortals _array_element))))
        ;[0 0 0 0.5] If trigger is to enable or disable portals in level.
        (for _array_element_2 (Variables|JustSpawnPortals?|GetPortalsToActivate)
          (switch Utilities|FlowControl|Switch|SwitchonEnum_ExitOrEnter (Variables|Setup|GetType%20of%20Trigger)
            (:NewEnumerator0
              (Default|DisablePortals _array_element_2))
            (:NewEnumerator1
              (Default|EnablePortals _array_element_2)
              ;;[0.1146 0.1146 0.1146 0.5] Sets the original transforms of the portal in case it's a rotatable portal.
              (Transformation|SetActorTransform _array_element_2 (Variables|/Gateweaver-PMS_v2/Plugin/BP_Portal.BP_Portal_C|GetOriginalTransform _array_element_2))))))
      (:then_1
        ;[0 0 0 0.5] If trigger is for portal gun as well, detach gun then set its transform back to its original spot
        (if (Variables|Setup|GetbHasPortalGun?)
          (bind _bp_gunref (Variables|PortalGun|GetBP_GunRef)
            (:then
              (Default|DropGun _bp_gunref)
              (Utilities|FlowControl|DelayUntilNextTick) ; i'm not quite sure if this is the correct node but it works
              (Transformation|SetActorTransform _bp_gunref (Variables|/Gateweaver-PMS_v2/Plugin/BP_Gun.BP_Gun_C|GetOriginalTransform _bp_gunref)))
            (:else)))))))

(event EventBeginPlay
  ;[0 0 0 0.5] Get all portal actors in scene and filter out the portals to spawn, so that by default it only removes portals that aren't needed.
  (CallFunction|GetAllPortalsinScene))

(fn ConstructionScript)

(fn GetAllPortalsinScene
  (bind _outactors (Actor|GetAllActorsOfClass "/Gateweaver-PMS_v2/Plugin/BP_Portal.BP_Portal_C"))
  (bind _output_get (Variables|Internal|SetAll%20Portals%20In%20Scene _outactors))
  (for _array_element _output_get
    (if (not (Utilities|Array|ContainsItem (Variables|JustSpawnPortals?|GetPortalsToActivate) _array_element))
      (Utilities|Array|Add (Variables|Internal|GetFilteredPortals) _array_element))))
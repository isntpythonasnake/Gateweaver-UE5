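; Portal gun pickup that attaches to the player on overlap and, while long-interacted, follows camera aim, locks movement and fires traces on a timer.
; Placement requires a Portal Passthrough surface, five-point flatness traces and no overlapping portal; rejected hits can play a colour-matched Niagara effect.
; SpawnPortalEvent scales out and destroys the gun's previous portal, then spawns its replacement, linking it to ExitPortal with a scale-up animation when one exists.
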(event OnComponentBeginOverlap(Box)
  (params (OverlappedComponent :type Primitive%20Component%20Object%20Reference) (OtherActor :type Actor%20Object%20Reference) (OtherComp :type Primitive%20Component%20Object%20Reference) (OtherBodyIndex :type Integer) (bFromSweep :type Boolean) (SweepResult :type Hit%20Result%20Structure%20%28by%20ref%29))
  (bind _returnvalue (Game|GetPlayerCharacter 0))
  ;[0 0 0 0.5] Attach gun to character socket
  (if (== _returnvalue OtherActor)
    (Transformation|AttachComponentToComponent (Variables|/Script/Engine.Character|GetMesh _returnvalue) (Variables|GunSetup|GetGun%20Socket) "SnapToTarget" "SnapToTarget" "KeepRelative" true)
    ;;[0.15 0.15 0.15 0.5] If character is not aiming, stop ignoring movement input
    (Input|ResetIgnoreMoveInput (Game|GetPlayerController 0))
    (Variables|Internal|SetisAIming false)))

(event OnLongInteraction(InteractionComponent)
  (params (Instigator :type Actor%20Object%20Reference) (Phase :type InteractionPhase%20Enum :default "NewEnumerator0") (Delta :type Float%20%28double-precision%29))
  ;[0 0 0 0.5] Spawn portals in set intervals after detaching from character to simulate aiming
  (switch Utilities|FlowControl|Switch|SwitchonInteractionPhase Phase
    (:NewEnumerator0
      (Transformation|DetachFromActor "KeepWorld" "KeepWorld" "KeepRelative")
      (bind _returnvalue (Utilities|Time|SetTimerbyEvent (delegate Custom|Intervals) (Variables|GunSetup|GetIntervalInSeconds) true))
      (Variables|Internal|SetTimer _returnvalue)
      (Input|SetIgnoreMoveInput (Game|GetPlayerController 0) true)
      (Variables|Internal|SetisAIming true))
    (:NewEnumerator3
      (Utilities|Time|ClearandInvalidateTimerbyHandle (Variables|Internal|GetTimer))
      ;[0 0 0 0.5] Attach gun to character socket
      (Transformation|AttachComponentToComponent (Variables|/Script/Engine.Character|GetMesh (Game|GetPlayerCharacter 0)) (Variables|GunSetup|GetGun%20Socket) "SnapToTarget" "SnapToTarget" "KeepRelative" true)
      ;;[0.15 0.15 0.15 0.5] If character is not aiming, stop ignoring movement input
      (Input|ResetIgnoreMoveInput (Game|GetPlayerController 0))
      (Variables|Internal|SetisAIming false))))

(event Custom|SpawnPortalEvent
  (params (Portal%20Transform :type Transform))
  ;[0 0 0 0.5] Portal spawn event for modularity - spawn from any actor, just use this actor as a variable
  ;;[0.09896 0.09896 0.09896 0.5] If an existing portal is spawned, destroy that portal with a scale down animation
  (Variables|Internal|SetbIsSpawned false)
  (Utilities|IsValid (Variables|Internal|GetSpawned%20Portal%20Object)
    (:Is%20Valid
      (Transformation|SetActorScale3D (Variables|Internal|GetSpawned%20Portal%20Object) "1.000000,1.000000,1.000000")
      (bind _scaleportal (Timeline|Timeline_0 ReverseFromEnd)
        (:Update
          (Transformation|SetActorScale3D (Variables|Internal|GetSpawned%20Portal%20Object) (Math|Conversions|ToVector(Float) _scaleportal)))
        (:Finished
          (Actor|DestroyActor (Variables|Internal|GetSpawned%20Portal%20Object))
          ;;[0.09896 0.09896 0.09896 0.5] Spawn new portal with a scale up animation and link it to the exit portal.
          (bind _returnvalue (Game|SpawnActorfromClass (Variables|Internal|GetPortal) Portal%20Transform "Undefined" "MultiplyWithRoot" 0 (Variables|PortalSetup|GetPanel%20Colour) (Variables|PortalSetup|GetPortal%20Frame%20Colour) (Variables|PortalSetup|GetbIsPanelHidden) 0 :!label _label))
          (bind _output_get (Variables|Internal|SetSpawned%20Portal%20Object _returnvalue))
          (Variables|Internal|SetbIsSpawned true)
          (Default|EnablePortals _output_get)
          (bind _exitportal (Variables|GunSetup|GetExitPortal)
            (:then
              (Variables|/Gateweaver-PMS_v2/Plugin/BP_Portal.BP_Portal_C|SetExit%20Portal _output_get _exitportal)
              (Transformation|SetActorScale3D _output_get "0, 0, 0")
              (bind _scaleportal_2 (Timeline|Timeline PlayFromStart)
                (:Update
                  (Transformation|SetActorScale3D _output_get (Math|Conversions|ToVector(Float) _scaleportal_2)))
                (:Finished
                  (Variables|/Script/Engine.SceneCaptureComponent2D|SetTextureTarget (Variables|/Gateweaver-PMS_v2/Plugin/BP_Portal.BP_Portal_C|GetPortalCamera (Variables|GunSetup|GetExitPortal)) (Variables|/Gateweaver-PMS_v2/Plugin/BP_Portal.BP_Portal_C|GetRender%20Target _output_get)))))
            (:else)))))
    (:Is%20Not%20Valid
      (goto _label))))

(event Custom|Intervals
  (bind _arrow (Variables|Default|GetArrow))
  (bind _returnvalue (Transformation|GetWorldLocation _arrow))
  ;[0 0 0 0.5] Spawn portals in set intervals after detaching from character to simulate aiming
  ;[0 0 0 0.5] Spawn portals using arrow as aim
  (bind _outhit (Collision|LineTraceByChannel _returnvalue (+ _returnvalue (* 5000 (Math|Vector|GetForwardVector (Transformation|GetWorldRotation _arrow)))) "TraceTypeQuery1" false 0 "None" true "(R=1.000000,G=0.000000,B=0.000000,A=1.000000)" "(R=0.000000,G=1.000000,B=0.000000,A=1.000000)" 0.0))
  ;[0 0 0 0.5] The values are hardcoded because while I may have improved in my math, I still haven't improved in math.
  (bind (_bisvalid _surfacelocation _surfacerotation) (CallFunction|ValidatePortalSurface _outhit 75.0 125.0 5.0 0.95 "TraceTypeQuery1"))
  ;[0 0 0 0.5] Spawn portal using an event
  (if _bisvalid
    (CallFunction|SpawnPortalEvent (Math|Transform|MakeTransform _surfacelocation _surfacerotation))))

(event Custom|DropGun
  ;[0 0 0 0.5] "Drops" gun
  (Transformation|DetachFromActor "KeepWorld" "KeepWorld" "KeepRelative"))

(event EventTick
  (params (DeltaSeconds :type Float%20%28single-precision%29))
  (bind _returnvalue (Game|GetPlayerCharacter 0))
  (bind _returnvalue_2 (Pawn|GetControlRotation _returnvalue :!class /Script/Engine.Pawn))
  ;[0 0 0 0.5] If the character is aiming, match gun rotation with camera's
  (if (Variables|Internal|GetisAIming)
    (Transformation|SetActorRotation (Math|Rotator|MakeRotator 0.0 (.pitch _returnvalue_2) (.yaw _returnvalue_2)))
    (Transformation|SetActorLocation (+ (Transformation|GetSocketLocation (Variables|/Script/Engine.Character|GetMesh _returnvalue) "Head") "0.000000,40.000000,40.000000") false false)))

(event EventBeginPlay
  ;[0 0 0 0.5] Get and store gun's original transform
  (Variables|Internal|SetOriginalTransform (Transformation|GetActorTransform)))

(fn ConstructionScript
  ;[0 0 0 0.5] Sets to whatever the gun mesh is
  (Components|StaticMesh|SetStaticMesh (Variables|Default|GetMesh) (Variables|GunSetup|GetGun%20Mesh))
  (Components|Activation|SetAutoActivate (Variables|Default|GetNS_InvalidPortal) false)
  ;[0 0 0 0.5] Sets the colour of the gun's effect thing to the colour of the gun's portal frame
  (bind _returnvalue (Rendering|Material|CreateDynamicMaterialInstance (Variables|Internal|GetPortal%20Frame%20Material) "Inst" "None" :!class /Script/Engine.KismetMaterialLibrary))
  (Rendering|Material|SetVectorParameterValue _returnvalue "Colour" (Variables|PortalSetup|GetPortal%20Frame%20Colour) :!class /Script/Engine.MaterialInstanceDynamic)
  (Rendering|Material|SetMaterial (Variables|Default|GetMesh) 1 _returnvalue))

(fn ValidatePortalSurface
  (params (HitResult :type Hit%20Result%20Structure) (PortalWidth :type Float%20%28double-precision%29) (PortalHeight :type Float%20%28double-precision%29) (SampleDistance :type Float%20%28double-precision%29) (NormalTolerance :type Float%20%28double-precision%29) (TraceChannel :type ETraceTypeQuery%20Enum :default "TraceTypeQuery1"))
  (bind (_bblockinghit _binitialoverlap _time _distance _location _impactpoint _normal _impactnormal) (Collision|BreakHitResult HitResult))
  (bind (_bblockinghit_2 _binitialoverlap_2 _time_2 _distance_2 _location_2 _impactpoint_2 _normal_2) (Collision|BreakHitResult HitResult))
  (bind (_bblockinghit_3 _binitialoverlap_3 _time_3 _distance_3 _location_3 _impactpoint_3 _normal_3 _impactnormal_2 _physmat _hitactor _hitcomponent) (Collision|BreakHitResult HitResult))
  (bind _returnvalue (Math|Rotator|MakeRotfromX _normal_3))
  (bind _returnvalue_2 (* SampleDistance _normal_3))
  (bind _returnvalue_3 (Math|Vector|GetRightVector _returnvalue))
  (bind _returnvalue_4 (Math|Vector|GetUpVector _returnvalue))
  (bind _returnvalue_5 (* _returnvalue_4 PortalHeight))
  (bind _returnvalue_6 (* _returnvalue_3 PortalWidth))
  ;[0 0 0 0.5] Noticed there's an error that claims the hit is null. this prevents it apparently.
  (if (!= _hitcomponent 0)
    ;[0 0 0 0.5] Detects surfaces for correct collision channel
    (switch Utilities|FlowControl|Switch|SwitchonECollisionChannel (Collision|GetCollisionObjectType _hitcomponent)
      (:ECC_WorldStatic
        (CallFunction|InvalidPortalEffects _location_2 _normal_2))
      (:ECC_GameTraceChannel1
        ;[0 0 0 0.5] Checks for flat surface and if surface has space to spawn portals.
        (for _array_element (Utilities|Array|MakeArray _location_3 (+ _location_3 _returnvalue_6 _returnvalue_5) (+ (- _location_3 _returnvalue_6) _returnvalue_5) (- (+ _location_3 _returnvalue_6) _returnvalue_5) (Utilities|Operators|Subtract _location_3 _returnvalue_6 _returnvalue_5))
          (bind (_outhit _returnvalue_7) (Collision|LineTraceByChannel (+ _array_element _returnvalue_2) (- _array_element _returnvalue_2) "TraceTypeQuery1" false 0 "None"))
          (if _returnvalue_7
            (if (not (>= (Math|Vector|DotProduct _normal_3 (.Normal (Collision|BreakHitResult _outhit))) NormalTolerance))
              (CallFunction|InvalidPortalEffects _location_2 _normal_2 :!label _label)
              ;[1 0.8429 0 0.5] If all is not well, do NOT spawn portal
              (bind _output_get (LocalVariables|SetbValid false))
              (return _output_get "0, 0, 0" "0, 0, 0"))
            (else
              (goto _label))))
        ;[0 0 0 0.5] Detects if there are any other portals in the vicinity of the portal, eg portals that already exist in the world.
        (bind _returnvalue_8 (Collision|BoxOverlapActors (+ _impactpoint (* _impactnormal 1e+01)) (Math|Vector|MakeVector (* PortalWidth 2.0) (* PortalHeight 0.6) 1e+02) (LocalVariables|GetObjectTypes) "/Gateweaver-PMS_v2/Plugin/BP_Portal.BP_Portal_C" :!class /Script/Engine.KismetSystemLibrary))
        (if _returnvalue_8
          (CallFunction|InvalidPortalEffects _location_2 _normal_2)
          (else
            ;;[0.06802 1 0 0.5] If all is well, spawn portal
            (bind _output_get_2 (LocalVariables|SetbValid true))
            (return _output_get_2 (+ (* (* PortalHeight -0.7) _returnvalue_4) (+ _location_3 (* _normal_3 6.0))) _returnvalue)))))
    (bind _output_get_3 (LocalVariables|SetbValid false))
    (return _output_get_3 "0, 0, 0" "0, 0, 0")))

(fn InvalidPortalEffects
  (params (Location :type Vector) (X :type Vector%20%28by%20ref%29))
  (bind _ns_invalidportal (Variables|Default|GetNS_InvalidPortal))
  ;[0 0 0 0.5] If portal gun is aimed at world static, set niagara effect to the colour of portal, then play it at hit loc of line trace
  (Transformation|SetWorldTransform _ns_invalidportal (Math|Transform|MakeTransform Location (Math|Rotator|MakeRotfromX X)) false false)
  (Niagara|SetNiagaraVariable(LinearColor) _ns_invalidportal "Particle Colour" (Variables|PortalSetup|GetPortal%20Frame%20Colour))
  (Components|Activation|Activate _ns_invalidportal false))
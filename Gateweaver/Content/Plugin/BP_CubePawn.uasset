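; Cube pawn that the player can pick up and carry by holding the interact key.
; On a started long interaction it moves to a collapsed-graph location, attaches to the player character and ignores Pawn collision.
; Cancelling detaches it and restores physics, gravity and blocking on all channels.
; Construction and BeginPlay make the cube block a custom trace channel, and BeginPlay also calls CubeIsSpawned.
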(event OnLongInteraction(InteractionComponent)
  (params (Instigator :type Actor%20Object%20Reference) (Phase :type InteractionPhase%20Enum :default "NewEnumerator0") (Delta :type Float%20%28double-precision%29))
  (bind _cube (Variables|Default|GetCube))
  (switch Utilities|FlowControl|Switch|SwitchonInteractionPhase Phase
    (:NewEnumerator0
      ;[0 0 0 0.5] Attach cube to player when player holds down interact key
      (Transformation|SetActorLocation (|CollapseGraph) false false)
      (Transformation|AttachActorToActor (Game|GetPlayerCharacter 0) "None" "KeepWorld" "KeepWorld" "KeepRelative" true)
      (Collision|SetCollisionResponsetoChannel (Variables|Default|GetCube) "ECC_Pawn" "ECR_Ignore"))
    (:NewEnumerator3
      ;[0 0 0 0.5] Detach when stop interacting
      (Physics|SetSimulatePhysics _cube true)
      (Physics|SetEnableGravity _cube true)
      (Transformation|DetachFromActor "KeepRelative" "KeepRelative" "KeepRelative")
      (Collision|SetCollisionResponsetoAllChannels _cube "ECR_Block"))))

(event EventBeginPlay
  (Collision|SetCollisionResponsetoChannel (Variables|Default|GetCube) "ECC_GameTraceChannel2" "ECR_Block")
  (Default|CallCubeIsSpawned))

(fn ConstructionScript
  (Collision|SetCollisionResponsetoChannel (Variables|Default|GetCube) "ECC_GameTraceChannel2" "ECR_Block"))
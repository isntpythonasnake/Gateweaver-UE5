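; Portal gun that attaches to the player's GunSocket on overlap and places a portal on the aimed surface.
; A held long interaction runs a looping timer that traces along the Arrow until cancelled.
; ValidatePortalSurface checks center and corner traces for a flat surface and rejects overlapping portals.
; Valid hits shrink out the previous portal, spawn a replacement and, given an ExitPortal, link it, scale it in and retarget the exit camera.
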(event OnComponentBeginOverlap(Box)
  (params (OverlappedComponent :type Primitive%20Component%20Object%20Reference) (OtherActor :type Actor%20Object%20Reference) (OtherComp :type Primitive%20Component%20Object%20Reference) (OtherBodyIndex :type Integer) (bFromSweep :type Boolean) (SweepResult :type Hit%20Result%20Structure%20%28by%20ref%29))
  (bind _returnvalue (Game|GetPlayerCharacter 0))
  ;[0 0 0 0.5] Attach gun to character socket
  (if (== _returnvalue OtherActor)
    (Transformation|AttachComponentToComponent (Variables|/Script/Engine.Character|GetMesh _returnvalue) (Variables|Default|GetGun%20Socket) "SnapToTarget" "KeepRelative" "KeepRelative" true)))

(event OnLongInteraction(InteractionComponent)
  (params (Instigator :type Actor%20Object%20Reference) (Phase :type InteractionPhase%20Enum :default "NewEnumerator0") (Delta :type Float%20%28double-precision%29))
  (switch Utilities|FlowControl|Switch|SwitchonInteractionPhase Phase
    (:NewEnumerator0
      (bind _returnvalue (Utilities|Time|SetTimerbyEvent (delegate Custom|Intervals) 1.0 true))
      (Variables|Default|SetTimer _returnvalue))
    (:NewEnumerator3
      (Utilities|Time|ClearandInvalidateTimerbyHandle (Variables|Default|GetTimer)))))

(event Custom|Intervals
  (bind _arrow (Variables|Default|GetArrow))
  (bind _returnvalue (Transformation|GetWorldLocation _arrow))
  ;[0 0 0 0.5] Spawn portals using arrow as aim
  (bind _outhit (Collision|LineTraceByChannel _returnvalue (+ _returnvalue (* 5000 (Math|Vector|GetForwardVector (Transformation|GetWorldRotation _arrow)))) "TraceTypeQuery1" false 0 "None" true "(R=1.000000,G=0.000000,B=0.000000,A=1.000000)" "(R=0.000000,G=1.000000,B=0.000000,A=1.000000)" 0.0))
  (bind (_bisvalid _surfacerotation _surfacelocation) (CallFunction|ValidatePortalSurface _outhit 75.0 125.0 5.0 0.95 "TraceTypeQuery1"))
  (if _bisvalid
    (Variables|Default|SetbIsSpawned false)
    (Utilities|IsValid (Variables|Default|GetSpawned%20Portal%20Object)
      (:Is%20Valid
        (Transformation|SetActorScale3D (Variables|Default|GetSpawned%20Portal%20Object) "1.000000,1.000000,1.000000")
        (bind _scaleportal (Timeline|Timeline_0 ReverseFromEnd)
          (:Update
            (Transformation|SetActorScale3D (Variables|Default|GetSpawned%20Portal%20Object) (Math|Conversions|ToVector(Float) _scaleportal)))
          (:Finished
            (Actor|DestroyActor (Variables|Default|GetSpawned%20Portal%20Object))
            (bind _returnvalue_2 (Game|SpawnActorfromClass (Variables|Default|GetPortal) (Math|Transform|MakeTransform _surfacelocation _surfacerotation) "Undefined" "MultiplyWithRoot" 0 (Variables|Default|GetPanel%20Colour) (Variables|Default|GetPortal%20Frame%20Colour) (Variables|Default|GetbIsPanelHidden) 0 :!label _label))
            (bind _output_get (Variables|Default|SetSpawned%20Portal%20Object _returnvalue_2))
            (Variables|Default|SetbIsSpawned true)
            (bind _exitportal (Variables|Default|GetExitPortal)
              (:then
                (Variables|/Game/Base/Plugin/PortalSource/Plugin/BP_Portal.BP_Portal_C|SetExit%20Portal _output_get _exitportal)
                (Default|EnablePortals _output_get)
                (Transformation|SetActorScale3D _output_get "0, 0, 0")
                (bind _scaleportal_2 (Timeline|Timeline PlayFromStart)
                  (:Update
                    (Transformation|SetActorScale3D _output_get (Math|Conversions|ToVector(Float) _scaleportal_2)))
                  (:Finished
                    (Variables|/Script/Engine.SceneCaptureComponent2D|SetTextureTarget (Variables|/Game/Base/Plugin/PortalSource/Plugin/BP_Portal.BP_Portal_C|GetPortalCamera (Variables|Default|GetExitPortal)) (Variables|/Game/Base/Plugin/PortalSource/Plugin/BP_Portal.BP_Portal_C|GetRender%20Target _output_get)))))
              (:else)))))
      (:Is%20Not%20Valid
        (goto _label)))))

(event EventBeginPlay
  (bind _returnvalue (Actor|GetActorOfClass (Variables|Default|GetPlayerCharacter)))
  (Variables|Default|SetPlayerCharacterActor _returnvalue))

(fn ConstructionScript)

(fn ValidatePortalSurface
  (params (HitResult :type Hit%20Result%20Structure) (PortalWidth :type Float%20%28double-precision%29) (PortalHeight :type Float%20%28double-precision%29) (SampleDistance :type Float%20%28double-precision%29) (NormalTolerance :type Float%20%28double-precision%29) (TraceChannel :type ETraceTypeQuery%20Enum :default "TraceTypeQuery1"))
  (bind (_bblockinghit _binitialoverlap _time _distance _location _impactpoint _normal _impactnormal) (Collision|BreakHitResult HitResult))
  (bind _returnvalue (* PortalHeight -0.7))
  (bind _returnvalue_2 (Math|Rotator|MakeRotfromX _normal))
  (bind _returnvalue_3 (* SampleDistance _normal))
  (bind _returnvalue_4 (* _normal 6.0))
  (bind _returnvalue_5 (Math|Vector|GetRightVector _returnvalue_2))
  (bind _returnvalue_6 (Math|Vector|GetUpVector _returnvalue_2))
  (bind _returnvalue_7 (+ _location _returnvalue_4))
  (bind _returnvalue_8 (* _returnvalue_6 PortalHeight))
  (bind _returnvalue_9 (* _returnvalue_5 PortalWidth))
  (bind _returnvalue_10 (* _returnvalue _returnvalue_6))
  (bind _returnvalue_11 (+ _returnvalue_10 _returnvalue_7))
  (for _array_element (Utilities|Array|MakeArray _location (+ _location _returnvalue_9 _returnvalue_8) (+ (- _location _returnvalue_9) _returnvalue_8) (- (+ _location _returnvalue_9) _returnvalue_8) (Utilities|Operators|Subtract _location _returnvalue_9 _returnvalue_8))
    (bind (_outhit _returnvalue_12) (Collision|LineTraceByChannel (+ _array_element _returnvalue_3) (Utilities|Operators|Subtract _array_element _returnvalue_3) "TraceTypeQuery1" false 0 "ForDuration"))
    (if _returnvalue_12
      (if (not (>= (Math|Vector|DotProduct _normal (.Normal (Collision|BreakHitResult _outhit))) NormalTolerance))
        (bind _output_get (LocalVariables|SetbValid false))
        (return _output_get _returnvalue_2 _returnvalue_11))
      (else
        (bind _output_get_2 (LocalVariables|SetbValid false))
        (return _output_get_2 _returnvalue_2 _returnvalue_11))))
  (bind _returnvalue_13 (Collision|BoxOverlapActors (+ _impactpoint (* _impactnormal 1e+01)) (Math|Vector|MakeVector (* PortalWidth 2.0) (* PortalHeight 0.6) 1e+02) (LocalVariables|GetObjectTypes) "/Game/Base/Plugin/PortalSource/Plugin/BP_Portal.BP_Portal_C" :!class /Script/Engine.KismetSystemLibrary))
  (if _returnvalue_13
    (bind _output_get_3 (LocalVariables|SetbValid false))
    (return _output_get_3 _returnvalue_2 _returnvalue_11)
    (else
      (bind _output_get_4 (LocalVariables|SetbValid true))
      (return _output_get_4 _returnvalue_2 _returnvalue_11))))
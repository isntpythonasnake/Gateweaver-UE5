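; BP_PhysicsButton is a button that reacts to actors other than the first player character overlapping its capsule.
; Begin overlap plays a timeline that drives the button mesh's relative Z location, and end overlap reverses it, without counting remaining overlaps.
; The button only animates itself, as its camera manager blend and deactivate logic is never run.
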(event OnComponentBeginOverlap(Capsule)
  (params (OverlappedComponent :type Primitive%20Component%20Object%20Reference) (OtherActor :type Actor%20Object%20Reference) (OtherComp :type Primitive%20Component%20Object%20Reference) (OtherBodyIndex :type Integer) (bFromSweep :type Boolean) (SweepResult :type Hit%20Result%20Structure%20%28by%20ref%29))
  (if (not (== OtherActor (Game|GetPlayerCharacter 0)))
    (bind _buttonmovement (Timeline|Timeline Play)
      (:Update
        (Transformation|SetRelativeLocation (Variables|Default|GetStaticMesh1) (Math|Vector|MakeVector 0.0 0.0 _buttonmovement) false false)))))

(event OnComponentEndOverlap(Capsule)
  (params (OverlappedComponent :type Primitive%20Component%20Object%20Reference) (OtherActor :type Actor%20Object%20Reference) (OtherComp :type Primitive%20Component%20Object%20Reference) (OtherBodyIndex :type Integer))
  (if (not (== OtherActor (Game|GetPlayerCharacter 0)))
    (bind _buttonmovement (Timeline|Timeline Reverse)
      (:Update
        (Transformation|SetRelativeLocation (Variables|Default|GetStaticMesh1) (Math|Vector|MakeVector 0.0 0.0 _buttonmovement) false false)))))

(fn ConstructionScript)
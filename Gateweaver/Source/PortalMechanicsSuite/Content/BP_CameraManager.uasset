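; Camera manager actor that blends player 0's view to requested camera positions and back to the controlled pawn.
; QueueBlend stores a transform and blend time in a single pending slot, overwriting any earlier request.
; On Tick, a pending request moves this actor to that transform and starts a cubic view-target blend to itself with the outgoing view locked.
; DeactivateCamera blends back to the pawn and clears any pending request.
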(event Custom|DeactivateCamera
  (params (BlendTime :type Float%20%28double-precision%29))
  (bind _returnvalue (Game|GetPlayerController 0))
  ;[0.15 0.15 0.15 0.5] Blend camera back to player and removes it from the queue.
  (Game|Player|SetViewTargetwithBlend _returnvalue (Pawn|GetControlledPawn _returnvalue) BlendTime "VTBlend_Linear" 0.0 false)
  (Variables|Default|SetbPendingBlend false))

(event Custom|QueueBlend
  (params (TargetTransform :type Transform) (BlendTime :type Float%20%28double-precision%29))
  ;[0.15 0.15 0.15 0.5] Queue camera requests
  ; - Call this event when activating camera.
  (Variables|Default|SetbPendingBlend true)
  (Variables|Default|SetTarget%20Transform TargetTransform)
  (Variables|Default|SetBlend%20Time BlendTime))

(event EventTick
  (params (DeltaSeconds :type Float%20%28single-precision%29))
  ;[0.15 0.15 0.15 0.5] Will only activate camera blend if no other blends are happening.
  (if (Variables|Default|GetbPendingBlend)
    ;[0.15 0.15 0.15 0.5] Set the position of the camera to be the arrow in the other actor
    (Transformation|SetActorTransform (Variables|Default|GetTarget%20Transform))
    (Game|Player|SetViewTargetwithBlend (Game|GetPlayerController 0) self (Variables|Default|GetBlend%20Time) "VTBlend_Cubic" 0.1 true)
    (Variables|Default|SetbPendingBlend false)))

(fn ConstructionScript)
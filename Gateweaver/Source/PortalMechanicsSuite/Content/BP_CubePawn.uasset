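; BP_CubePawn is a cube the player picks up and carries through a long interaction on its InteractionComponent.
; Starting the interaction attaches it to the player character, positions it once ahead of the camera at CarryDistance with an upward offset, and ignores Pawn collision.
; Cancelling re-enables physics and gravity, detaches it and blocks all channels.
; Construction and BeginPlay block a custom trace channel, and BeginPlay also calls CubeIsSpawned.
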(event OnLongInteraction(InteractionComponent)
  (params (Instigator :type Actor%20Object%20Reference) (Phase :type InteractionPhase%20Enum :default "NewEnumerator0") (Delta :type Float%20%28double-precision%29))
  (bind _returnvalue (Game|GetPlayerCameraManager 0))
  (bind _cube (Variables|Default|GetCube))
  (bind _returnvalue_2 (Camera|GetCameraRotation _returnvalue))
  (switch Utilities|FlowControl|Switch|SwitchonInteractionPhase Phase
    (:NewEnumerator0
      (Transformation|AttachActorToActor (Game|GetPlayerCharacter 0) "None" "SnapToTarget" "SnapToTarget" "KeepRelative" true)
      (Transformation|SetActorLocation (+ (Math|Vector|GetUpVector _returnvalue_2) (+ (* (Math|Vector|GetForwardVector _returnvalue_2) (Variables|Default|GetCarryDistance)) (Camera|GetCameraLocation _returnvalue))) false false)
      (Collision|SetCollisionResponsetoChannel _cube "ECC_Pawn" "ECR_Ignore"))
    (:NewEnumerator3
      (Physics|SetSimulatePhysics _cube true)
      (Physics|SetEnableGravity _cube true)
      (Transformation|DetachFromActor "KeepRelative" "KeepRelative" "KeepRelative")
      (Collision|SetCollisionResponsetoAllChannels _cube "ECR_Block"))))

(event EventBeginPlay
  (Collision|SetCollisionResponsetoChannel (Variables|Default|GetCube) "ECC_GameTraceChannel2" "ECR_Block")
  (Default|CallCubeIsSpawned))

(fn ConstructionScript
  (Collision|SetCollisionResponsetoChannel (Variables|Default|GetCube) "ECC_GameTraceChannel2" "ECR_Block"))